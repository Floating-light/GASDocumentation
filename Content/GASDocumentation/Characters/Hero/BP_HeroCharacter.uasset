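; Hero character Blueprint from the GAS documentation project, whose graph holds debug logic for monitoring Meteor ability gameplay effects.
; Five seconds after BeginPlay, the authority starts an async listener on its Ability System Component for GE_MeteorCost being added or removed.
; Each event prints to screen, labeled as Meteor cooldown despite watching the cost effect.
; An unconnected cooldown-tag listener for Ability5 never runs.
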(event `self.ReceiveBeginPlay`
  (`KismetSystemLibrary.Delay` 5.0)
  (`/Engine/EditorBlueprintResources/ActorMacros.Switch Has Authority`
    (:`Authority`
      (`AsyncGEAddedRemoved.ListenForGEAddedRemoved` (`AbilitySystemBlueprintLibrary.GetAbilitySystemComponent` self) "/Game/GASDocumentation/Characters/Hero/Abilities/Meteor/GE_MeteorCost.GE_MeteorCost_C"
        (:`then`
          (`KismetSystemLibrary.PrintString` (`KismetStringLibrary.Concat_StrStr` (`KismetSystemLibrary.GetDisplayName` self) "===BindGE class listen in server ") true true (struct :`G` 0.66 :`B` 1.0 :`A` 1.0) 50.0))
        (:`OnGEAdded`
          (`KismetSystemLibrary.PrintString` (`KismetStringLibrary.Concat_StrStr` (`KismetSystemLibrary.GetDisplayName` self) "====Server ------>> Add GE Meteor CoolDown") true true (struct :`G` 0.66 :`B` 1.0 :`A` 1.0) 50.0))
        (:`OnGERemoved`
          (`KismetSystemLibrary.PrintString` (`KismetStringLibrary.Concat_StrStr` (`KismetSystemLibrary.GetDisplayName` self) "====Server ------>> Remove GE Meteor CoolDown") true true (struct :`G` 0.66 :`B` 1.0 :`A` 1.0) 50.0))))))

(event `self.ReceiveTick`
  (params (DeltaSeconds :type "Float (single-precision)")))

(fn `UserConstructionScript`)